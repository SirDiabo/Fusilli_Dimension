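; Pickup item that grants the player one of four buffs by BuffType: speed, damage, double score or fire-rate change.
; Overlap with PlayerBP hides and disables the item, applies the buff, then destroys the actor, after a delay except for fire rate.
; Only double score is reverted after the delay; other stat changes persist, and fire rate scales GunSHot's play rate.
; Tick, throttled by a Delay, colors the Niagara effect by buff type.
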(event OnComponentBeginOverlap(Sphere)
  (params (OverlappedComponent :type Primitive%20Component%20Object%20Reference) (OtherActor :type Actor%20Object%20Reference) (OtherComp :type Primitive%20Component%20Object%20Reference) (OtherBodyIndex :type Integer) (bFromSweep :type Boolean) (SweepResult :type Hit%20Result%20Structure%20%28by%20ref%29))
  (bind _asplayer_bp (Utilities|Casting|CastToPlayerBP OtherActor))
  (if (not (Variables|Default|GetDisabled?))
    (CallFunction|DisableBuff)
    (switch Utilities|FlowControl|Switch|Switchonenum_BuffTypes (Variables|Default|GetBuff%20Type)
      (:NewEnumerator0
        (Variables|/Script/Engine.CharacterMovementComponent|SetMaxWalkSpeed (Variables|/Script/Engine.Character|GetCharacterMovement _asplayer_bp) (+ (Variables|/Script/Engine.CharacterMovementComponent|GetMaxWalkSpeed (Variables|/Script/Engine.Character|GetCharacterMovement _asplayer_bp)) 1e+02))
        (Utilities|FlowControl|Delay 3e+01))
      (:NewEnumerator1
        (Variables|/Game/Blueprints/PlayerBP.PlayerBP_C|SetDamage _asplayer_bp (+ (Variables|/Game/Blueprints/PlayerBP.PlayerBP_C|GetDamage _asplayer_bp) 0.1))
        (Utilities|FlowControl|Delay 3e+01))
      (:NewEnumerator2
        (Variables|/Game/Blueprints/PlayerBP.PlayerBP_C|SetDouble%20Score? _asplayer_bp true)
        (Utilities|FlowControl|Delay 3e+01)
        (bind _asplayer_bp_2 (Utilities|Casting|CastToPlayerBP (Game|GetPlayerCharacter 0)))
        (Variables|/Game/Blueprints/PlayerBP.PlayerBP_C|SetDouble%20Score? _asplayer_bp_2 false))
      (:NewEnumerator3
        (Components|Timeline|SetPlayRate (Variables|/Game/Blueprints/PlayerBP.PlayerBP_C|GetGun%20SHot _asplayer_bp) (* (Components|Animation|GetPlayRate (Variables|/Game/Blueprints/PlayerBP.PlayerBP_C|GetGun%20SHot _asplayer_bp)) 0.8))))
    (Actor|DestroyActor)))

(event Custom|Disable%20Buff
  (Variables|Default|SetDisabled? true)
  (Rendering|SetVisibility (Variables|Default|GetStaticMesh) false false)
  (Components|Activation|Deactivate (Variables|Default|GetNiagara)))

(event EventTick
  (params (DeltaSeconds :type Float%20%28single-precision%29))
  (Utilities|FlowControl|Delay 1.0)
  (Effects|Components|ParticleSystem|SetColorParameter (Variables|Default|GetNiagara) "Color" (Utilities|Select :Index (Variables|Default|GetBuff%20Type) :NewEnumerator0 "(R=0.000000,G=0.000000,B=1.000000,A=1.000000)" :NewEnumerator1 "(R=1.000000,G=0.000000,B=0.000000,A=1.000000)" :NewEnumerator2 "(R=0.000000,G=1.000000,B=0.000000,A=1.000000)" :NewEnumerator3 "(R=1.000000,G=1.000000,B=0.000000,A=1.000000)")))

(fn ConstructionScript)