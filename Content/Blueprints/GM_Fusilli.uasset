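; Game mode for Fusilli that applies saved player settings and manages dynamic graphics scalability.
; On BeginPlay it sets scalability and copies camera and weapon sway settings from the game instance's save game to the player.
; If the save enables dynamic scalability, a Delay-throttled Tick samples frame rate and steps the level down when low or up when high.
; Scalability is issued by console command, with an animated HUD message naming the level.
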(event Custom|Set%20Scalability
  (Development|ExecuteConsoleCommand (Utilities|String|Append "scalability " (Utilities|String|ToString(Integer) (Variables|Default|GetScalability%20Reference))) 0)
  (bind _ashud_fusilli (Utilities|Casting|CastToHUD_Fusilli (HUD|GetHUD (Game|GetPlayerController 0))))
  (Utilities|IsValid (Variables|/Game/Blueprints/HUD_Fusilli.HUD_Fusilli_C|GetWidget%20Reference _ashud_fusilli)
    (:Is%20Valid
      (UserInterface|Animation|PlayAnimation (Variables|/Game/Blueprints/HUD_Fusilli.HUD_Fusilli_C|GetWidget%20Reference _ashud_fusilli) (Variables|/Game/Blueprints/PlayerWidget.PlayerWidget_C|GetScalabilityMessage (Variables|/Game/Blueprints/HUD_Fusilli.HUD_Fusilli_C|GetWidget%20Reference _ashud_fusilli)) 0.0 1 "Forward" 1.0 false)
      (Rendering|Components|TextRender|SetText (Variables|/Game/Blueprints/PlayerWidget.PlayerWidget_C|GetScalabilityText (Variables|/Game/Blueprints/HUD_Fusilli.HUD_Fusilli_C|GetWidget%20Reference _ashud_fusilli)) (Utilities|Text|FormatText "Scalability changed to \"{scalability option}\"" (Utilities|Select :Index (Variables|Default|GetScalability%20Reference) :Option%200 "LOW" :Option%201 "MEDIUM" :Option%202 "HIGH" :Option%203 "EXTREME" :Option%204 "ULTRA"))))))

(event Custom|Update%20Settings
  (bind _as_gi_fusilli (Variables|Default|GetAs%20GI%20Fusilli))
  (bind _as_save_game_bp (Variables|/Game/Blueprints/GI_Fusilli.GI_Fusilli_C|GetAs%20Save%20Game%20BP _as_gi_fusilli))
  (Utilities|FlowControl|Sequence
    (:then_0
      (Variables|/Game/Blueprints/PlayerBP.PlayerBP_C|SetCamera%20Sensitivity (Variables|Default|GetAs%20Player%20BP) (Variables|/Game/Blueprints/SaveGameBP.SaveGameBP_C|GetCamera%20Sensitivity _as_save_game_bp)))
    (:then_1
      (Variables|/Game/Blueprints/PlayerBP.PlayerBP_C|SetCamera%20Roll%20Strengh (Variables|Default|GetAs%20Player%20BP) (Variables|/Game/Blueprints/SaveGameBP.SaveGameBP_C|GetCamera%20Roll%20Strengh _as_save_game_bp)))
    (:then_2
      (Variables|/Game/Blueprints/PlayerBP.PlayerBP_C|SetWeapon%20Upsway (Variables|Default|GetAs%20Player%20BP) (Variables|/Game/Blueprints/SaveGameBP.SaveGameBP_C|GetWeapon%20Upsway%20Strengh _as_save_game_bp)))))

(event EventBeginPlay
  (bind _asgi_fusilli (Utilities|Casting|CastToGI_Fusilli (Game|GetGameInstance)))
  (Variables|Default|SetAs%20GI%20Fusilli _asgi_fusilli)
  (bind _asplayer_bp (Utilities|Casting|CastToPlayerBP (Game|GetPlayerCharacter 0)))
  (Variables|Default|SetAs%20Player%20BP _asplayer_bp)
  (CallFunction|SetScalability)
  (CallFunction|UpdateSettings))

(event EventTick
  (params (DeltaSeconds :type Float%20%28single-precision%29))
  (bind _returnvalue (Utilities|Time|GetWorldDeltaSeconds))
  (bind _returnvalue_2 (/ 1.0 _returnvalue))
  (Utilities|FlowControl|Sequence
    (:then_0
      (if (Variables|/Game/Blueprints/SaveGameBP.SaveGameBP_C|GetDynamic%20Scalability (Variables|/Game/Blueprints/GI_Fusilli.GI_Fusilli_C|GetAs%20Save%20Game%20BP (Variables|Default|GetAs%20GI%20Fusilli)))
        (Utilities|FlowControl|Delay 0.5)
        (if (< _returnvalue_2 4e+01)
          (Variables|Default|SetScalability%20Reference (Math|Integer|Clamp(Integer) (- (Variables|Default|GetScalability%20Reference) 1) 0 4))
          (CallFunction|SetScalability :!label _label)
          (elif (>= _returnvalue_2 1.2e+02)
            (Variables|Default|SetScalability%20Reference (Math|Integer|Clamp(Integer) (+ (Variables|Default|GetScalability%20Reference) 1) 0 4))
            (goto _label)))))))

(fn ConstructionScript)