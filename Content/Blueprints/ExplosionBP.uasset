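; Explosion actor that plays a grenade pop sound and effect when Boom fires, then destroys itself when its timeline ends.
; The timeline scales a sphere, whose overlaps launch players away from the center and deal lethal-scale damage to skeletons.
; The skeleton launch direction uses the explosion's location as both endpoints, so its launch velocity resolves to zero.
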(event OnComponentBeginOverlap(Sphere)
  (params (OverlappedComponent :type Primitive%20Component%20Object%20Reference) (OtherActor :type Actor%20Object%20Reference) (OtherComp :type Primitive%20Component%20Object%20Reference) (OtherBodyIndex :type Integer) (bFromSweep :type Boolean) (SweepResult :type Hit%20Result%20Structure%20%28by%20ref%29))
  (Utilities|FlowControl|Sequence
    (:then_0
      (bind _asplayer_bp (Utilities|Casting|CastToPlayerBP OtherActor))
      (Character|LaunchCharacter _asplayer_bp (* (Math|Vector|GetUnitDirection(Vector) (Transformation|GetActorLocation) (Transformation|GetActorLocation _asplayer_bp)) 1500) true true))
    (:then_1
      (bind _asskeleton_bp (Utilities|Casting|CastToSkeletonBP OtherActor))
      (Character|LaunchCharacter _asskeleton_bp (* (Math|Vector|GetUnitDirection(Vector) (Transformation|GetActorLocation) (Transformation|GetActorLocation)) 1500) true true)
      (Default|TakeDamage _asskeleton_bp 999.0))))

(event Custom|Boom
  (Audio|PlaySoundatLocation "/Game/SFX/Grenade_Pop.Grenade_Pop" (Transformation|GetActorLocation) "0, 0, 0" 1.0 1.0 0.0 "/Game/SFX/NewSoundAttenuation1.NewSoundAttenuation1" 0 0 0)
  (Niagara|SpawnSystematLocation "/Game/VFX/PS_Grenade_Explode.PS_Grenade_Explode" (Transformation|GetActorLocation))
  (bind _newtrack_0 (Timeline|Timeline_0 PlayFromStart)
    (:Update
      (Transformation|SetWorldScale3D (Variables|Default|GetSphere) (Math|Conversions|ToVector(Float) _newtrack_0)))
    (:Finished
      (Actor|DestroyActor))))

(fn ConstructionScript)