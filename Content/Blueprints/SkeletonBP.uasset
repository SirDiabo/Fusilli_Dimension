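; Skeleton enemy that chases the nearest PlayerBP and randomly chooses a melee montage or a cooldown-gated leap attack.
; Tick drives targeting, AIMoveTo and attacks, with a DoOnce serializing attacks.
; Mid-leap overlaps damage players and other skeletons, while hits received then deal lethal damage.
; Authority-triggered death ragdolls it, awards player 0 score and a grenade, saves any new highscore, then destroys it.
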(event OnSeePawn(PawnSensing)
  (params (Pawn :type Pawn%20Object%20Reference))
  (Utilities|Casting|CastToPlayerBP Pawn)
  (Variables|Default|SetStates "NewEnumerator1"))

(event OnComponentBeginOverlap(Capsule)
  (params (OverlappedComponent :type Primitive%20Component%20Object%20Reference) (OtherActor :type Actor%20Object%20Reference) (OtherComp :type Primitive%20Component%20Object%20Reference) (OtherBodyIndex :type Integer) (bFromSweep :type Boolean) (SweepResult :type Hit%20Result%20Structure%20%28by%20ref%29))
  (bind _is_air_attacking (Variables|Default|GetIs%20Air%20Attacking))
  (bind _health (Variables|Default|GetHealth))
  (bind _returnvalue (> _health 0.0))
  (bind _returnvalue_2 (and _returnvalue _is_air_attacking))
  (Utilities|FlowControl|Sequence
    (:then_0
      (bind _asplayer_bp (Utilities|Casting|CastToPlayerBP OtherActor))
      (if _returnvalue_2
        (Default|TakeDamage _asplayer_bp 2.0 1.0)))
    (:then_1
      (if (!= OtherActor self)
        (bind _asskeleton_bp (Utilities|Casting|CastToSkeletonBP OtherActor))
        (if (Variables|Default|GetCan%20Damage%20other%20skeleton)
          (if _returnvalue_2
            (CallFunction|TakeDamage _asskeleton_bp 3.0)
            (Variables|Default|SetCan%20Damage%20other%20skeleton false)
            (Utilities|FlowControl|Delay 5.0)
            (Variables|Default|SetCan%20Damage%20other%20skeleton true)))))))

(event Custom|Check%20if%20Dead%20and%20Kill%20tell%20all
  (CallFunction|CheckifDeadandKill))

(event Custom|Check%20If%20Dead%20and%20Kill%20tell%20server
  (CallFunction|CheckifDeadandKillTellAll))

(event Custom|Delete%20Actor%20After%20Death
  (Utilities|FlowControl|Delay 5.0)
  (Actor|DestroyActor))

(event EventOnLanded
  (params (Hit :type Hit%20Result%20Structure%20%28by%20ref%29))
  (bind _scene_hitparticle (Variables|Default|GetScene_HitParticle))
  (bind _returnvalue (Transformation|GetWorldTransform _scene_hitparticle))
  (Variables|Default|SetIsDashing? false)
  (Utilities|FlowControl|Delay 1.45)
  (Variables|Default|SetIs%20Air%20Attacking false)
  (Variables|/Script/Engine.CharacterMovementComponent|SetMaxWalkSpeed (Variables|Character|GetCharacterMovement) 5.5e+02)
  (Utilities|FlowControl|Sequence
    (:then_0
      (Utilities|FlowControl|Delay 5.0)
      (Variables|Default|SetCanDash true))
    (:then_1
      (Utilities|FlowControl|DoOnce false) ; enters at Reset
    )))

(event EventHit
  (params (Damage :type Float%20%28double-precision%29))
  (if (Variables|Default|GetIs%20Air%20Attacking)
    (CallFunction|TakeDamage 999.0)
    (else
      (CallFunction|TakeDamage Damage))))

(event EventBeginPlay
  (bind _asgi_fusilli (Utilities|Casting|CastToGI_Fusilli (Game|GetGameInstance)))
  (Variables|Default|SetAs%20GI%20Fusilli _asgi_fusilli))

(event EventTick
  (params (DeltaSeconds :type Float%20%28single-precision%29))
  (bind _scene_hitparticle (Variables|Default|GetScene_HitParticle))
  (bind _returnvalue (Transformation|GetWorldTransform _scene_hitparticle))
  (Utilities|FlowControl|Sequence
    (:then_0
      (Utilities|FlowControl|Delay 0.1)
      (if (<= (Variables|Default|GetHealth) 0.0)
        (Utilities|FlowControl|DoOnce false
          (:Completed
            (Networking|SwitchHasAuthority
              (:Authority
                (CallFunction|CheckifDeadandKillTellAll)))))))
    (:then_1
      (Utilities|FlowControl|Delay 0.1)
      (Variables|Default|SetDistance%20to%20player 999.0)
      (bind _outactors (Actor|GetAllActorsOfClass "/Game/Blueprints/PlayerBP.PlayerBP_C"))
      (for _array_element _outactors
        (if (< (Math|Vector|Distance(Vector) (Transformation|GetActorLocation _array_element) (Transformation|GetActorLocation)) (Variables|Default|GetDistance%20to%20player))
          (Variables|Default|SetDistance%20to%20player (Math|Vector|Distance(Vector) (Transformation|GetActorLocation _array_element) (Transformation|GetActorLocation)))
          (Variables|Default|SetTarget%20Player _array_element)))
      (AI|AIMoveTo self "0, 0, 0" (Variables|Default|GetTarget%20Player) 1e+02 false
        (:then
          (Utilities|FlowControl|DoOnce false :!label _label
            (:Completed
              (if (<= (CallFunction|DistancefromPlayer) 2e+02)
                (if (Math|Random|RandomBool)
                  (Animation|PlayAnimMontage "/Game/Mesh/Skeleton/AM_Skeleton_Attack.AM_Skeleton_Attack" 1.0 "None" :!label _label_2)
                  (Utilities|FlowControl|Delay 0.6)
                  (if (<= (CallFunction|DistancefromPlayer) 2e+02)
                    (if (> (Variables|Default|GetHealth) 0.0)
                      (bind _asplayer_bp (Utilities|Casting|CastToPlayerBP (Game|GetPlayerCharacter 0)))
                      (Default|TakeDamage _asplayer_bp 1.0 1.0)
                      (Effects|SpawnEmitteratLocation 0 (.location _returnvalue) (.rotation _returnvalue))
                      (goto _label Reset)
                      (else
                        (goto _label Reset)))
                    (else
                      (goto _label Reset)))
                  (elif (Variables|Default|GetCanDash)
                    (Variables|Default|SetCanDash false)
                    (Variables|Default|SetIsDashing? true)
                    (Variables|/Script/Engine.CharacterMovementComponent|SetMaxWalkSpeed (Variables|Character|GetCharacterMovement) 0.0)
                    (Utilities|FlowControl|Delay 1.0)
                    (Variables|Default|SetIs%20Air%20Attacking true)
                    (Character|LaunchCharacter (* (Transformation|GetActorUpVector) 1000) false false)
                    (Utilities|FlowControl|Delay 0.2)
                    (Character|LaunchCharacter (* (Transformation|GetActorForwardVector) 1000) false false)
                    (else
                      (goto _label_2))))
                (else
                  (goto _label Reset))))))))))

(fn ConstructionScript)

(fn CheckifDeadandKill
  (bind _mesh (Variables|Character|GetMesh))
  (bind _as_gi_fusilli (Variables|Default|GetAs%20GI%20Fusilli))
  (bind _as_save_game_bp (Variables|/Game/Blueprints/GI_Fusilli.GI_Fusilli_C|GetAs%20Save%20Game%20BP _as_gi_fusilli))
  (Utilities|FlowControl|Sequence
    (:then_0
      (Collision|SetCollisionEnabled (Variables|Collision|GetCapsuleComponent) "NoCollision"))
    (:then_1
      (Collision|SetCollisionEnabled _mesh "QueryAndPhysics"))
    (:then_2
      (Components|Animation|SetAnimationMode _mesh "AnimationSingleNode"))
    (:then_3
      (Components|Animation|PlayAnimation _mesh 0 false))
    (:then_4
      (Physics|SetSimulatePhysics _mesh true))
    (:then_5
      (Variables|Default|SetCanDoDamage? false))
    (:then_6
      (CallFunction|DeleteActorAfterDeath))
    (:then_7
      (bind _asplayer_bp (Utilities|Casting|CastToPlayerBP (Game|GetPlayerCharacter 0)))
      (bind _output_get (Variables|/Game/Blueprints/PlayerBP.PlayerBP_C|SetScore _asplayer_bp (+ (Variables|/Game/Blueprints/PlayerBP.PlayerBP_C|GetScore _asplayer_bp) (select (Variables|/Game/Blueprints/PlayerBP.PlayerBP_C|GetDouble%20Score? _asplayer_bp) 2.0 1.0))))
      (Default|AddGrenade _asplayer_bp)
      (if (> _output_get (Variables|/Game/Blueprints/SaveGameBP.SaveGameBP_C|GetHighscore _as_save_game_bp))
        (Variables|/Game/Blueprints/SaveGameBP.SaveGameBP_C|SetHighscore _as_save_game_bp _output_get)
        (SaveGame|SaveGametoSlot _as_save_game_bp (Variables|/Game/Blueprints/GI_Fusilli.GI_Fusilli_C|GetSave%20Name _as_gi_fusilli))))))

(fn TakeDamage
  (params (Damage :type Float%20%28double-precision%29))
  (Variables|Default|SetHealth (Math|Float|Clamp(Float) (- (Variables|Default|GetHealth) Damage) 0.0 5.0)))

(fn DistancefromPlayer
  (bind _target_player (Variables|Default|GetTarget%20Player))
  (Utilities|IsValid _target_player
    (:Is%20Valid
      (return (Math|Vector|Distance(Vector) (Transformation|GetActorLocation _target_player) (Transformation|GetActorLocation))))
    (:Is%20Not%20Valid
      (return 9999999999.0))))