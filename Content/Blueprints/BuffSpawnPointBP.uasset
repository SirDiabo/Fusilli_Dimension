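; Spawn point actor for random player buff pickups.
; ActivateItem marks the point active, spawns a buff item of one of four random types (speed, damage, double score, fire rate) at its transform and starts its Niagara effect.
; An unwired chain, which never runs, would disable the item, apply its buff to PlayerBP, revert it after a delay and then free the point.
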(event Custom|Activate%20Item
  (Variables|Default|SetActive true)
  (bind _returnvalue (Game|SpawnActorfromClass "/Game/Blueprints/BuffItemBP.BuffItemBP_C" (Transformation|GetActorTransform) "Undefined" 0 (Utilities|Select :Index (Math|Random|RandomIntegerinRange 0 3) :Option%200 "NewEnumerator0" :Option%201 "NewEnumerator1" :Option%202 "NewEnumerator2" :Option%203 "NewEnumerator3") 0))
  (bind _output_get (Variables|Default|SetSpawned%20Item _returnvalue))
  (Components|Activation|Activate (Variables|/Game/Blueprints/BuffItemBP.BuffItemBP_C|GetNiagara _output_get) true)
  (Development|PrintString "Spawned"))

(fn ConstructionScript)