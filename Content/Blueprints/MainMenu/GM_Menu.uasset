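; Main menu game mode that applies the player's saved graphics and audio settings on BeginPlay.
; It caches the Fusilli game instance and player pawn, stopping if either cast fails, then runs UpdateSettings from the instance's save game.
; UpdateSettings sets console scalability unless dynamic scalability is on, drives PSX shader color and resolution through a material parameter collection, and overrides main sound class volume.
; SetScalability is called but empty.
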(event Custom|Update%20Settings
  (bind _as_gi_fusilli (Variables|Default|GetAs%20GI%20Fusilli))
  (bind _as_save_game_bp (Variables|/Game/Blueprints/GI_Fusilli.GI_Fusilli_C|GetAs%20Save%20Game%20BP _as_gi_fusilli))
  (Utilities|FlowControl|Sequence
    (:then_0
      (if (not (Variables|/Game/Blueprints/SaveGameBP.SaveGameBP_C|GetDynamic%20Scalability _as_save_game_bp))
        (Development|ExecuteConsoleCommand (Utilities|String|Append "scalability " (Utilities|String|ToString(Integer) (Variables|/Game/Blueprints/SaveGameBP.SaveGameBP_C|GetScalability%20Index _as_save_game_bp))) 0)))
    (:then_1
      (Rendering|Material|SetScalarParameterValue "/Game/Materials/Postprocess/MaterialParameterCollection_PSXShader.MaterialParameterCollection_PSXShader" "Color Intensity" (Variables|/Game/Blueprints/SaveGameBP.SaveGameBP_C|GetColor%20Scale _as_save_game_bp) :!class /Script/Engine.KismetMaterialLibrary))
    (:then_2
      (Rendering|Material|SetScalarParameterValue "/Game/Materials/Postprocess/MaterialParameterCollection_PSXShader.MaterialParameterCollection_PSXShader" "Resolution Scale" (Variables|/Game/Blueprints/SaveGameBP.SaveGameBP_C|GetResolution%20Scale _as_save_game_bp) :!class /Script/Engine.KismetMaterialLibrary))
    (:then_3
      (Audio|SetSoundMixClassOverride "/Game/SFX/SMM_Main.SMM_Main" "/Game/SFX/SC_Main.SC_Main" (Variables|/Game/Blueprints/SaveGameBP.SaveGameBP_C|GetVolume _as_save_game_bp) 1.0 0.0 true))))

(event EventBeginPlay
  (bind _asgi_fusilli (Utilities|Casting|CastToGI_Fusilli (Game|GetGameInstance)))
  (Variables|Default|SetAs%20GI%20Fusilli _asgi_fusilli)
  (bind _asplayer_bp (Utilities|Casting|CastToPlayerBP (Game|GetPlayerCharacter 0)))
  (Variables|Default|SetAs%20Player%20BP _asplayer_bp)
  (CallFunction|SetScalability)
  (CallFunction|UpdateSettings))

(fn ConstructionScript)

(fn SetScalability)