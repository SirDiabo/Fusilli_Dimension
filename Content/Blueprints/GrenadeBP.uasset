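; Grenade actor that explodes on contact with the world, pawns or physics objects, ignoring the player.
; Each Tick runs a small sphere trace at its own location in place of collision events.
; The first valid hit passes a DoOnce, spawns an ExplosionBP there, calls its Boom and destroys the grenade.
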(event EventTick
  (params (DeltaSeconds :type Float%20%28single-precision%29))
  (bind _returnvalue (Transformation|GetActorLocation))
  (bind (_outhit _returnvalue_2) (Collision|SphereTraceForObjects _returnvalue _returnvalue 32.0 (Utilities|Array|MakeArray "ObjectTypeQuery1" "ObjectTypeQuery3" "ObjectTypeQuery2" "ObjectTypeQuery4") false (Utilities|Array|MakeArray (Variables|Default|GetPlayer%20Reference)) "None"))
  (if (and (!= (.HitActor (Collision|BreakHitResult _outhit)) "/Game/Blueprints/PlayerBP.PlayerBP") _returnvalue_2)
    (Utilities|FlowControl|DoOnce false
      (:Completed
        (bind _returnvalue_3 (Game|SpawnActorfromClass "/Game/Blueprints/ExplosionBP.ExplosionBP_C" (Math|Transform|MakeTransform (Transformation|GetActorLocation) "0, 0, 0" "1.000000,1.000000,1.000000") "Undefined" 0 0))
        (Default|Boom _returnvalue_3)
        (Actor|DestroyActor)))))

(fn ConstructionScript)